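; BP_PieceSpawner spawns random pieces over the player's position on a looping timer started at BeginPlay.
; SpawnPiece requires a valid PlayingArea and traces vertically through the player's capsule on Visibility.
; A hit places a PieceOptions actor at the hit component's X and Y, raised HeightToSpawn above the impact.
; Each spawn attempt multiplies SpawningInterval by Multiplieramount, but the running timer is never reset with the new value.
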(event Custom|SpawnPiece
  (bind _pieceoptions (Variables|Default|GetpieceOptions))
  (Utilities|IsValid (Variables|Default|GetplayingArea)
    (:Is%20Valid
      (Variables|Default|SetspawningInterval (* (Variables|Default|GetspawningInterval) (Variables|Default|Getmultiplieramount)))
      (bind _aspapertestcharacter (Utilities|Casting|CastTopapertestcharacter (Game|GetPlayerCharacter 0)))
      (bind (_outhit _returnvalue) (Collision|LineTraceByChannel (+ (Transformation|GetWorldLocation (Variables|/Script/Engine.Character|GetCapsuleComponent _aspapertestcharacter)) "0.000000,0.000000,3000.000000") (+ (Transformation|GetWorldLocation (Variables|/Script/Engine.Character|GetCapsuleComponent _aspapertestcharacter)) (* (* (Math|Vector|GetUpVector (Variables|/Script/Engine.Character|GetCapsuleComponent _aspapertestcharacter)) -1.0) "0.000000,0.000000,500.000000")) "TraceTypeQuery1" false 0 "None"))
      (if _returnvalue
        (Game|SpawnActorfromClass (Utilities|Array|Get(acopy) _pieceoptions (Math|Random|RandomInteger (- (Utilities|Array|Length _pieceoptions) 1))) (Math|Transform|MakeTransform (Math|Vector|MakeVector (.X (Math|Vector|BreakVector (Transformation|GetWorldLocation (.HitComponent (Collision|BreakHitResult _outhit))))) (.Y (Math|Vector|BreakVector (Transformation|GetWorldLocation (.HitComponent (Collision|BreakHitResult _outhit))))) (+ (.Z (Math|Vector|BreakVector (.Location (Collision|BreakHitResult _outhit)))) (Variables|Default|GetheightToSpawn))) "0, 0, 0" "1.000000,1.000000,1.000000") "Undefined" "MultiplyWithRoot" 0 0)))))

(event EventBeginPlay
  (bind _returnvalue (Utilities|Time|SetTimerbyEvent (EventDispatchers|CreateEvent :!event Custom|SpawnPiece) (Variables|Default|GetspawningInterval) true))
  (Variables|Default|SetspawningTimer _returnvalue))

(fn ConstructionScript)