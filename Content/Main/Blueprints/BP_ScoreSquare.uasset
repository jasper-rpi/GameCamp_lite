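; BP_ScoreSquare is a score pickup whose Pillow mesh jumps to random spots on the BP_PlayingArea.
; MovePoint line-traces from above to below randomly picked area meshes, retrying until it hits the area or a stationary BP_Piece; a complete miss leaves it in place.
; Overlap by papertestcharacter calls GetScore and relocates it, while overlap by a BP_Piece only relocates it.
; DepthPass toggles the Pillow's custom depth rendering.
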(event OnComponentBeginOverlap(pillow)
  (params (OverlappedComponent :type Primitive%20Component%20Object%20Reference) (OtherActor :type Actor%20Object%20Reference) (OtherComp :type Primitive%20Component%20Object%20Reference) (OtherBodyIndex :type Integer) (bFromSweep :type Boolean) (SweepResult :type Hit%20Result%20Structure%20%28by%20ref%29))
  (bind _aspapertestcharacter (Utilities|Casting|CastTopapertestcharacter OtherActor)
    (:then
      (Default|GetScore _aspapertestcharacter)
      (CallFunction|MovePoint))
    (:CastFailed
      (Utilities|Casting|CastToBP_Piece OtherActor)
      (CallFunction|MovePoint))))

(event Custom|movePoint
  (Utilities|FlowControl|Sequence
    (:then_0
      (Utilities|IsValid (Variables|Default|GetplayingArea)
        (:Is%20Valid
          (bind _asbp_playing_area (Utilities|Casting|CastToBP_PlayingArea (Variables|Default|GetplayingArea)))
          (bind (_outhit _returnvalue) (Collision|LineTraceByChannel (+ (Transformation|GetWorldLocation (Utilities|Array|Get(acopy) (Variables|/Game/Main/Blueprints/BP_PlayingArea.BP_PlayingArea_C|GetplayingAreaMeshes _asbp_playing_area) (Math|Random|RandomIntegerinRange 0 (- (Utilities|Array|Length (Variables|/Game/Main/Blueprints/BP_PlayingArea.BP_PlayingArea_C|GetplayingAreaMeshes _asbp_playing_area)) 1)))) "0.000000,0.000000,2000.000000") (- (Transformation|GetWorldLocation (Utilities|Array|Get(acopy) (Variables|/Game/Main/Blueprints/BP_PlayingArea.BP_PlayingArea_C|GetplayingAreaMeshes _asbp_playing_area) (Math|Random|RandomIntegerinRange 0 (- (Utilities|Array|Length (Variables|/Game/Main/Blueprints/BP_PlayingArea.BP_PlayingArea_C|GetplayingAreaMeshes _asbp_playing_area)) 1)))) "0.000000,0.000000,100.000000") "TraceTypeQuery1" false 0 "None" :!label _label))
          (if _returnvalue
            (bind _asbp_piece (Utilities|Casting|CastToBP_Piece (.HitActor (Collision|BreakHitResult _outhit)))
              (:then
                (if (Variables|/Game/Main/Blueprints/BP_Piece.BP_Piece_C|GetisMoving _asbp_piece)
                  (Utilities|Casting|CastToBP_PlayingArea (.HitActor (Collision|BreakHitResult _outhit)) :!label _label_2
                    (:then
                      _)
                    (:CastFailed
                      (goto _label)))))
              (:CastFailed
                (goto _label_2)))
            (Transformation|SetWorldLocation (Variables|Default|Getpillow) (.Location (Collision|BreakHitResult _outhit)) false false)))))))

(event Custom|DepthPass
  (params (should%20DepthPass :type Boolean))
  (Rendering|SetRenderCustomDepth (Variables|Default|Getpillow) should%20DepthPass))

(event EventBeginPlay
  (CallFunction|MovePoint))

(fn ConstructionScript)