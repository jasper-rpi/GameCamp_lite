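; BP_ScoreSquare is a pickup marker that jumps to a new spot in the playing area whenever a papertestcharacter overlaps it.
; On BeginPlay and on each overlap, MovePoint line-traces from high above to randomly picked BP_PlayingArea meshes, leaving persistent debug lines.
; A hit moves the Cylinder component just above the impact point.
; The Blueprint itself awards no score.
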(event OnComponentBeginOverlap(Cylinder)
  (params (OverlappedComponent :type Primitive%20Component%20Object%20Reference) (OtherActor :type Actor%20Object%20Reference) (OtherComp :type Primitive%20Component%20Object%20Reference) (OtherBodyIndex :type Integer) (bFromSweep :type Boolean) (SweepResult :type Hit%20Result%20Structure%20%28by%20ref%29))
  (Utilities|Casting|CastTopapertestcharacter OtherActor)
  (CallFunction|MovePoint))

(event Custom|movePoint
  (Utilities|IsValid (Variables|Default|GetplayingArea)
    (:Is%20Valid
      (bind _asbp_playing_area (Utilities|Casting|CastToBP_PlayingArea (Variables|Default|GetplayingArea)))
      (bind (_outhit _returnvalue) (Collision|LineTraceByChannel (+ (Transformation|GetWorldLocation (Utilities|Array|Get(acopy) (Variables|/Game/Main/Blueprints/BP_PlayingArea.BP_PlayingArea_C|GetplayingAreaMeshes _asbp_playing_area) (Math|Random|RandomIntegerinRange 0 (- (Utilities|Array|Length (Variables|/Game/Main/Blueprints/BP_PlayingArea.BP_PlayingArea_C|GetplayingAreaMeshes _asbp_playing_area)) 1)))) "0.000000,0.000000,2000.000000") (Transformation|GetWorldLocation (Utilities|Array|Get(acopy) (Variables|/Game/Main/Blueprints/BP_PlayingArea.BP_PlayingArea_C|GetplayingAreaMeshes _asbp_playing_area) (Math|Random|RandomIntegerinRange 0 (- (Utilities|Array|Length (Variables|/Game/Main/Blueprints/BP_PlayingArea.BP_PlayingArea_C|GetplayingAreaMeshes _asbp_playing_area)) 1)))) "TraceTypeQuery1" false 0 "Persistent"))
      (if _returnvalue
        (Transformation|SetWorldLocation (Variables|Default|GetCylinder) (+ (.Location (Collision|BreakHitResult _outhit)) "0.000000,0.000000,50.000000") false false)))))

(event EventBeginPlay
  (CallFunction|MovePoint))

(fn ConstructionScript)