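; BP_Piece is a falling block piece that drops in fixed steps until it lands on something.
; A looping timer set on BeginPlay at the FallSpeed interval drives MovePieceDown, which moves the actor down 100 units per tick.
; Before each step, a short downward line trace from every static mesh component checks for WorldDynamic objects.
; A hit cancels the drop and clears the timer through a DoOnce.
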(event Custom|MovePieceDown
  (Variables|Default|SetshouldDrop true)
  (for _array_element (Actor|GetComponentsByClass "/Script/Engine.StaticMeshComponent")
    ;[1 1 1] check if hit something and cancel the drop if true
    (bind _returnvalue (Collision|LineTraceForObjects (Transformation|GetWorldLocation _array_element) (- (Transformation|GetWorldLocation _array_element) "0.000000,0.000000,50.000000") (Utilities|Array|MakeArray "ObjectTypeQuery2") false 0 "None"))
    (if _returnvalue
      (Utilities|FlowControl|DoOnce false
        (:Completed
          (Variables|Default|SetshouldDrop false)
          (Utilities|Time|ClearandInvalidateTimerbyHandle (Variables|Default|GetmovePieceTimer))))))
  ;[1 1 1] move actor down 100 units
  (if (Variables|Default|GetshouldDrop)
    (Transformation|AddActorLocalOffset "0.000000,0.000000,-100.000000" false false)))

(event EventBeginPlay
  (bind _returnvalue (Utilities|Time|SetTimerbyEvent (EventDispatchers|CreateEvent :!event Custom|MovePieceDown) (Variables|Default|GetfallSpeed) true))
  (Variables|Default|SetmovePieceTimer _returnvalue))

(fn ConstructionScript)