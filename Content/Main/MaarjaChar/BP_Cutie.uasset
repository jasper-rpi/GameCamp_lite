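; Player character BP_Cutie, with camera-relative walking, yaw rotation and jumping driven by Enhanced Input.
; BeginPlay adds the mapping context and a post-process component that fakes tilt-shift with shallow depth of field focused at spring arm length.
; Walk inputs store their axis values and move along camera vectors; sideways walking also prints a debug string.
; Jumping or walking off a ledge sends the PaperZD animation instance to its "air" node.
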(event Input|EnhancedActionEvents|EnhancedInputActionIA_rotate
  (params (ActionValue :type Float%20%28double-precision%29) (ElapsedSeconds :type Float%20%28double-precision%29) (TriggeredSeconds :type Float%20%28double-precision%29) (InputAction :type Input%20Action%20Object%20Reference :default "/Game/TestCharacter/IA_rotate.IA_rotate"))
  ;[0.08854 0.08854 0.08854 0.5] Pööra kaamerat
  (:Triggered
    (Pawn|Input|AddControllerYawInput ActionValue)))

(event Input|EnhancedActionEvents|EnhancedInputActionIA_Walk
  (params (ActionValue :type Float%20%28double-precision%29) (ElapsedSeconds :type Float%20%28double-precision%29) (TriggeredSeconds :type Float%20%28double-precision%29) (InputAction :type Input%20Action%20Object%20Reference :default "/Game/Main/Input/IA_Walk.IA_Walk"))
  ;[0.08854 0.08854 0.08854 0.5] kõnni edasi / tagasi
  (:Triggered
    (Variables|Default|SetwalkForwards ActionValue)
    (Pawn|Input|AddMovementInput (Math|Vector|GetForwardVector (Transformation|GetWorldRotation (Variables|Default|GetCamera))) ActionValue false)))

(event Input|EnhancedActionEvents|EnhancedInputActionIA_WalkSide
  (params (ActionValue :type Float%20%28double-precision%29) (ElapsedSeconds :type Float%20%28double-precision%29) (TriggeredSeconds :type Float%20%28double-precision%29) (InputAction :type Input%20Action%20Object%20Reference :default "/Game/Main/Input/IA_WalkSide.IA_WalkSide"))
  ;[0.08854 0.08854 0.08854 0.5] Kõnni paremale / vasakule
  (:Triggered
    (Variables|Default|SetWalkSideways ActionValue)
    (Development|PrintString "j")
    (Pawn|Input|AddMovementInput (Math|Vector|GetRightVector (Transformation|GetWorldRotation (Variables|Default|GetCamera))) ActionValue false)))

(event Input|EnhancedActionEvents|EnhancedInputActionJump
  (params (ActionValue :type Boolean) (ElapsedSeconds :type Float%20%28double-precision%29) (TriggeredSeconds :type Float%20%28double-precision%29) (InputAction :type Input%20Action%20Object%20Reference :default "/Game/TestCharacter/Jump.Jump"))
  ;[0.08854 0.08854 0.08854 0.5] hüpe
  (:Started
    (Character|Jump))
  (:Canceled
    (Character|StopJumping)))

(event EventBeginPlay
  ;[1 1 1] tiltshift
  (bind _returnvalue (AddComponent|AddPostProcessComponent false))
  (Utilities|Struct|SetmembersinPostProcessSettings (Variables|/Script/Engine.PostProcessComponent|GetSettings _returnvalue) 0.3 1.5e+02 (Variables|/Script/Engine.SpringArmComponent|GetTargetArmLength (Variables|Default|GetSpringArm)))
  (bind _asplayer_controller (Utilities|Casting|CastToPlayerController (Pawn|GetController)))
  (Input|AddMappingContext (PlayerController|LocalPlayerSubsystems|GetEnhancedInputLocalPlayerSubsystem _asplayer_controller) "/Game/TestCharacter/mappings.mappings" 0 "(bIgnoreAllPressedKeysUntilRelease=True,bForceImmediately=False)"))

(event EventOnJumped
  (Class|PaperZDAnimInstance|JumptoNode (Variables|/Script/PaperZD.PaperZDAnimationComponent|GetAnimInstance (Variables|Default|GetAnimationComponent)) "air" "None"))

(event EventOnWalkingOffLedge
  (params (PreviousFloorImpactNormal :type Vector%20%28by%20ref%29 :default "0, 0, 0") (PreviousFloorContactNormal :type Vector%20%28by%20ref%29 :default "0, 0, 0") (PreviousLocation :type Vector%20%28by%20ref%29 :default "0, 0, 0") (TimeDelta :type Float%20%28single-precision%29))
  (Class|PaperZDAnimInstance|JumptoNode (Variables|/Script/PaperZD.PaperZDAnimationComponent|GetAnimInstance (Variables|Default|GetAnimationComponent)) "air" "None"))

(fn ConstructionScript)