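; BP_PieceSpawner periodically spawns pieces above random spots in a playing area.
; BeginPlay starts a looping timer at SpawningInterval, apparently driving SpawnPiece.
; SpawnPiece casts PlayingArea to BP_PlayingArea, picks a random mesh from PlayingAreaMeshes and spawns PieceToSpawn at its location, raised by HeightToSpawn.
; The random index uses RandomInteger on array length minus one, so the last mesh is never chosen.
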(event Custom|SpawnPiece
  (Utilities|IsValid (Variables|Default|GetplayingArea)
    (:Is%20Valid
      ;[1 1 1] spawn the piece
      (bind _asbp_playing_area (Utilities|Casting|CastToBP_PlayingArea (Variables|Default|GetplayingArea)))
      (bind _output_get (Variables|Default|SetindexToSpawn (Math|Random|RandomInteger (- (Utilities|Array|Length (Variables|/Game/Main/Blueprints/BP_PlayingArea.BP_PlayingArea_C|GetplayingAreaMeshes _asbp_playing_area)) 1))))
      (Game|SpawnActorfromClass (Variables|Default|GetpieceToSpawn) (Math|Transform|MakeTransform (Math|Vector|MakeVector (.X (Math|Vector|BreakVector (Transformation|GetWorldLocation (Utilities|Array|Get(acopy) (Variables|/Game/Main/Blueprints/BP_PlayingArea.BP_PlayingArea_C|GetplayingAreaMeshes _asbp_playing_area) _output_get)))) (.Y (Math|Vector|BreakVector (Transformation|GetWorldLocation (Utilities|Array|Get(acopy) (Variables|/Game/Main/Blueprints/BP_PlayingArea.BP_PlayingArea_C|GetplayingAreaMeshes _asbp_playing_area) _output_get)))) (+ (.Z (Math|Vector|BreakVector (Transformation|GetWorldLocation (Utilities|Array|Get(acopy) (Variables|/Game/Main/Blueprints/BP_PlayingArea.BP_PlayingArea_C|GetplayingAreaMeshes _asbp_playing_area) _output_get)))) (Variables|Default|GetheightToSpawn))) "0, 0, 0" "1.000000,1.000000,1.000000") "Undefined" "MultiplyWithRoot" 0 0))))

(event EventBeginPlay
  (bind _returnvalue (Utilities|Time|SetTimerbyEvent (EventDispatchers|CreateEvent :!event Custom|SpawnPiece) (Variables|Default|GetspawningInterval) true))
  (Variables|Default|SetspawningTimer _returnvalue))

(fn ConstructionScript)