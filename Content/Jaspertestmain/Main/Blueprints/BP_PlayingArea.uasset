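; BP_PlayingArea is a grid floor for the playing area whose tiles can be tinted red as a warning indicator.
; The Construction Script builds the row-by-column grid of static mesh components, spaced by MeshDimension, and stores them in PlayingAreaMeshes.
; ChangeMaterial applies a new red dynamic material instance to a given component when indicating.
; Otherwise it recolors only the last stored instance dark gray, ignoring the component passed in.
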(event EventChangeMaterial
  (params (shouldIndicate :type Boolean) (component :type Primitive%20Component%20Object%20Reference))
  (if shouldIndicate
    (bind _returnvalue (Rendering|Material|CreateDynamicMaterialInstance "/Game/Main/Material/BaseColors/M_SimpleColor.M_SimpleColor" "None" "None" :!class /Script/Engine.KismetMaterialLibrary))
    (bind _output_get (Variables|Default|SetMI_WarningMaterial _returnvalue))
    (Rendering|Material|SetVectorParameterValue _output_get "Color" "(R=0.718750,G=0.000000,B=0.000000,A=1.000000)" :!class /Script/Engine.MaterialInstanceDynamic)
    (Rendering|Material|SetMaterial component 0 (Variables|Default|GetMI_WarningMaterial))
    (else
      (Rendering|Material|SetVectorParameterValue (Variables|Default|GetMI_WarningMaterial) "Color" "(R=0.088542,G=0.088542,B=0.088542,A=1.000000)" :!class /Script/Engine.MaterialInstanceDynamic))))

(fn ConstructionScript
  (for _index (range 0 (- (* (Variables|Default|GetareaRow) (Variables|Default|GetareaCol)) 1))
    (Variables|Default|SetcurrentIndex _index)
    (bind _returnvalue (AddComponent|AddStaticMeshComponent false (Math|Transform|MakeTransform (Math|Vector|MakeVector (* (/ (Variables|Default|GetcurrentIndex) (Variables|Default|GetareaCol)) (Variables|Default|GetmeshDimension)) (* (Math|Integer|%(Integer) (Variables|Default|GetcurrentIndex) (Variables|Default|GetareaCol)) (Variables|Default|GetmeshDimension)) 0.0) "0, 0, 0" "1.000000,1.000000,1.000000")))
    (Components|StaticMesh|SetStaticMesh _returnvalue (Variables|Default|GetmeshToDisplay))
    (Utilities|Array|Add (Variables|Default|GetplayingAreaMeshes) _returnvalue)
    (Rendering|Material|SetMaterial _returnvalue 0 (Variables|Default|GetmaterialToUse))))